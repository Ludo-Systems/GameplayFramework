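; GA_GainMana is a Gameplay Ability that restores the owner's mana through the GE_ResetPlayerMana gameplay effect.
; On activation it commits first, then compares current mana to max mana on the avatar's attribute component and applies the effect only if below max.
; Because the commit precedes that check, activating at full mana still commits the ability.
; Every path ends the ability immediately.
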(event Ability|EventActivateAbility
  (bind _returnvalue (Ability|GetAvatarActorfromActorInfo))
  (bind _returnvalue_2 (Class|DaAttributeComponent|FindAttributeComponent _returnvalue))
  (bind _returnvalue_3 (Ability|CommitAbility))
  (if _returnvalue_3
    (if (< (Class|DaAttributeComponent|GetMana _returnvalue_2) (Class|DaAttributeComponent|GetMaxMana _returnvalue_2))
      (Ability|ApplyGameplayEffectToOwner "/Game/GlitchShaper/AbilitySystem/Effects/GE_ResetPlayerMana.GE_ResetPlayerMana_C")
      (Ability|EndAbility)
      (else
        (Ability|EndAbility :!label _label)))
    (else
      (goto _label))))