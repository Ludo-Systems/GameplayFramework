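; GA_MeleeAttack is a Gameplay Ability that performs a short forward dash followed by a melee strike.
; After committing, it applies a brief root motion force along the avatar's forward vector with a dash montage, then switches to the attack montage.
; During the attack it waits for a single Event.Damage gameplay event and applies GE_DealDamage to the payload target with a set-by-caller Damage magnitude.
; The ability ends after the hit or montage completion.
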(event Ability|EventActivateAbility
  (bind _returnvalue (Ability|CommitAbility))
  (if _returnvalue
    (Ability|Tasks|ApplyRootMotionConstantForce "None" (Transformation|GetActorForwardVector (Ability|GetAvatarActorfromActorInfo)) 1e+01 0.1 false 0 "MaintainLastRootMotionVelocity"
      (:then
        (|PlayMontageandWaitProxy "None" (Variables|Default|GetDashAnim) 1.0 "None" true 1.0 0.0 false))
      (:OnFinish
        (Animation|Montage|MontageStop -1.0)
        (|PlayMontageandWaitProxy "None" (Variables|Default|GetAttackAnim) 1.0 "None" true 1.0 0.0 false
          (:then
            (bind _payload (Ability|Tasks|WaitGameplayEvent "(TagName=\"Event.Damage\")" 0 true)
              (:EventReceived
                (bind _returnvalue_2 (Ability|GameplayEffect|AssignTagSetbyCallerMagnitude (Ability|MakeOutgoingGameplayEffectSpec "/Game/GlitchShaper/AbilitySystem/Effects/GE_DealDamage.GE_DealDamage_C") "(TagName=\"Event.Damage\")" (Variables|Default|GetDamage)))
                (GameplayEffects|ApplyGameplayEffectSpecToTarget (Ability|GetAbilitySystemComponent (Ability|GetAvatarActorfromActorInfo)) _returnvalue_2 (Ability|GetAbilitySystemComponent (.Target (Utilities|Struct|BreakGameplayEventData _payload))))
                (Ability|EndAbility))))
          (:OnCompleted
            (Ability|EndAbility)))))
    (else
      (Ability|EndAbility))))

(event Ability|EventOnEndAbility
  (params (bWasCancelled :type Boolean))
  (Development|PrintString "End Ability Melee Attack"))