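; GA_Buff_Thorns is a gameplay ability that reflects a fraction of incoming damage back at the attacker.
; Triggered by a damage event, it skips cases where the avatar is the instigator, since both sides receive that event.
; It divides the event magnitude by a divisor, clamps and rounds it, then passes it as SetByCaller damage to GE_DamageThorns.
; The event's Target applies that effect to the Instigator, and the ability ends.
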(event Ability|EventActivateAbilityFromEvent
  (params (EventData :type Gameplay%20Event%20Data%20Structure%20%28by%20ref%29))
  (if (!= (Ability|GetAvatarActorfromActorInfo) (.instigator EventData))
    (bind _returnvalue (Ability|GameplayEffect|AssignTagSetbyCallerMagnitude (Ability|MakeOutgoingGameplayEffectSpec "/Game/GlitchShaper/AbilitySystem/Effects/GE_DamageThorns.GE_DamageThorns_C") "(TagName=\"Gameplay.Damage\")" (CallFunction|CaclulateFractionalDamage (.eventmagnitude EventData))))
    (GameplayEffects|ApplyGameplayEffectSpecToTarget (Ability|GetAbilitySystemComponent (.target EventData)) _returnvalue (Ability|GetAbilitySystemComponent (.instigator EventData))) ; Swap Target and instigator since Thorns abilities want to damage the instigator
    (Ability|EndAbility)
    (else
      (Ability|EndAbility))))

(fn CaclulateFractionalDamage
  (params (IncomingDamage :type Float%20%28double-precision%29))
  (return (Math|Conversions|ToFloat(Integer) (Math|Float|Round (Math|Float|Clamp(Float) (/ IncomingDamage (Variables|Default|GetDamageDivisor)) 1.0 (Variables|Default|GetMaxThornsDamage))))))