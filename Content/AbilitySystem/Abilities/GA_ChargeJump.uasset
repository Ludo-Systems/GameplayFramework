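; Gameplay ability for a charged jump that plays a charging montage while timing player input, via either a second press or button release.
; On input, it stops the montage, applies a root motion jump force along avatar rotation plus GE_Jump, and ends on landing.
; CalculateJumpForceFromTime scales distance, height and duration from charge time, though its inverted Min/Max clamp never returns less than MaxChargeTime.
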(event Ability|EventActivateAbility
  (bind (_distance _height _duration) (CallFunction|CalculateJumpForcefromTime))
  (bind _returnvalue (Ability|CommitAbility))
  (if _returnvalue
    (|PlayMontageandWaitProxy "None" (Variables|Default|GetChargingJumpMontage) 1.0 "None" true 1.0 0.0 false ; HACK: Set an animation state to trigger a charging Jump animation which will play until the jump animation fires
      (:then
        (if (Variables|Default|GetbEnableDoublePress)
          (bind _timewaited (Ability|Tasks|WaitInputPress false)
            (:OnPress
              (Variables|Default|SetCurrentChargeTime _timewaited)))
          (else
            (bind _timeheld (Ability|Tasks|WaitInputRelease false)
              (:OnRelease
                (Variables|Default|SetCurrentChargeTime _timeheld)))))
        (Animation|Montage|MontageStop -1.0)
        (|ApplyRootMotionJumpForce "None" (Transformation|GetActorRotation (Ability|GetAvatarActorfromActorInfo)) _distance _height _duration 0.0 true "MaintainLastRootMotionVelocity" "0, 0, 0" 0.0
          (:then
            (Ability|ApplyGameplayEffectToOwner "/Game/GlitchShaper/AbilitySystem/Effects/GE_Jump.GE_Jump_C"))
          (:OnLanded
            (Ability|EndAbility)))))
    (else
      (Ability|EndAbility))))

(event Ability|EventOnEndAbility
  (params (bWasCancelled :type Boolean))
  (Development|PrintString "End Charge Jump"))

(fn CalculateJumpForcefromTime
  (bind _minchargetime (Variables|Default|GetMinChargeTime))
  (bind _maxchargetime (Variables|Default|GetMaxChargeTime))
  (bind _currentchargetime (Variables|Default|GetCurrentChargeTime))
  (bind _returnvalue (Math|Float|Min(Float) _currentchargetime _minchargetime))
  (bind _returnvalue_2 (Math|Float|Max(Float) _returnvalue _maxchargetime))
  (return (* (Variables|Default|GetDistanceMultiplier) _returnvalue_2) (* _returnvalue_2 (Variables|Default|GetHeightMultiplier)) (* _returnvalue_2 (Variables|Default|GetDurationMulltiplier))))