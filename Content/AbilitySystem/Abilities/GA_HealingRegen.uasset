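; Gameplay ability that grants health regeneration to its owner.
; On activation it commits, then applies the GE_Regen effect unless the avatar's attribute component reports max health, and ends immediately in every case.
; The commit precedes the health check, so any cost or cooldown applies even at full health.
; A casting montage task is present but disconnected, so it never plays.
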(event Ability|EventActivateAbility
  (bind _returnvalue (Ability|CommitAbility))
  (if _returnvalue
    (if (Class|DaAttributeComponent|IsatMaxHealth (Class|DaAttributeComponent|FindAttributeComponent (Ability|GetAvatarActorfromActorInfo)))
      (Ability|EndAbility)
      (else
        (Ability|ApplyGameplayEffectToOwner "/Game/GlitchShaper/AbilitySystem/Effects/GE_Regen.GE_Regen_C")
        (Ability|EndAbility)))
    (else
      (Ability|EndAbility))))